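; BP_DTurret is a turret obstacle that spawns BP_Bullet projectiles and damages any Paper2D character that hits it.
; Tick drives firing through latent Delay nodes: a Start flag gives the first tick a one-second delay, and later ticks use the BulletTIme interval.
; Each completed delay spawns a bullet at the BulletSpawn component's world transform.
; The Hit event casts to PaperCharacter and applies fixed damage.
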(event EventTick
  (params (DeltaSeconds :type Float%20%28single-precision%29))
  (if (Variables|Default|GetStart)
    (Utilities|FlowControl|Delay (Variables|Default|GetBulletTIme))
    (else
      (Variables|Default|SetStart true)
      (Utilities|FlowControl|Delay 1.0)))
  (Game|SpawnActorfromClass "/Game/Blueprints/Obstacles/BP_Bullet.BP_Bullet_C" (Transformation|GetWorldTransform (Variables|Default|GetBulletSpawn)) "Undefined" 0 0))

(event Collision|EventHit
  (params (MyComp :type Primitive%20Component%20Object%20Reference) (Other :type Actor%20Object%20Reference) (OtherComp :type Primitive%20Component%20Object%20Reference) (bSelfMoved :type Boolean) (HitLocation :type Vector :default "0, 0, 0") (HitNormal :type Vector :default "0, 0, 0") (NormalImpulse :type Vector :default "0, 0, 0") (Hit :type Hit%20Result%20Structure%20%28by%20ref%29))
  (bind _aspaper_character (Utilities|Casting|CastToPaperCharacter Other))
  (Game|Damage|ApplyDamage _aspaper_character 3.0 0 0))

(fn ConstructionScript)