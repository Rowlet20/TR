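; BP_HEnemie1 is a horizontal patrol enemy that damages any PaperCharacter it hits.
; Each Tick it adds movement input along X in the direction set by LookingR and rotates to face that way.
; It records its starting X once, derives right and left limits from MaxRight and MaxLeft offsets, and flips LookingR on reaching either limit.
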(event EventTick
  (params (DeltaSeconds :type Float%20%28single-precision%29))
  (Utilities|FlowControl|Sequence
    (:then_0
      (Pawn|Input|AddMovementInput "1.000000, 0,0.000000" (select (Variables|Default|GetLookingR) 1.0 -1.0) false))
    (:then_1
      (if (Variables|Default|GetOriginalPositionB)
        (Variables|Default|SetOriginalPosition (.x (Transformation|GetActorLocation)))
        (Variables|Default|SetOriginalPositionB false)))
    (:then_2
      (if (Variables|Default|GetLookingR)
        (if (Variables|Default|GetFirstPos)
          (Variables|Default|SetFirstPos false)
          (bind _output_get (Variables|Default|SetPositionR (+ (Variables|Default|GetOriginalPosition) (.x (Variables|Default|GetMaxRight))))))
        (if (>= (.x (Transformation|GetActorLocation)) _output_get)
          (Variables|Default|SetLookingR false)
          (Variables|Default|SetFirstPos true))
        (else
          (if (Variables|Default|GetFirstPos)
            (Variables|Default|SetFirstPos false)
            (bind _output_get_2 (Variables|Default|SetPositionL (- (Variables|Default|GetOriginalPosition) (* (.x (Variables|Default|GetMaxLeft)) -1.0)))))
          (if (<= (.x (Transformation|GetActorLocation)) _output_get_2)
            (Variables|Default|SetLookingR true)
            (Variables|Default|SetFirstPos false)))))
    (:then_3
      (if (Variables|Default|GetLookingR)
        (Transformation|SetActorRotation "0, 0, 0")
        (else
          (Transformation|SetActorRotation "0.000000,180.000000,0.000000"))))))

(event Collision|EventHit
  (params (MyComp :type Primitive%20Component%20Object%20Reference) (Other :type Actor%20Object%20Reference) (OtherComp :type Primitive%20Component%20Object%20Reference) (bSelfMoved :type Boolean) (HitLocation :type Vector :default "0, 0, 0") (HitNormal :type Vector :default "0, 0, 0") (NormalImpulse :type Vector :default "0, 0, 0") (Hit :type Hit%20Result%20Structure%20%28by%20ref%29))
  (bind _aspaper_character (Utilities|Casting|CastToPaperCharacter Other))
  (Game|Damage|ApplyDamage _aspaper_character 3.0 0 0))

(fn ConstructionScript)