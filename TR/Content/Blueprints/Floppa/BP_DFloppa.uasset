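; BP_DFloppa is a disappearing Floppa platform that also lets the player change gravity.
; A hit on the Cube plays a flipbook, then after a short delay hides the actor, disables Cube collision and plays a sound at world origin.
; Two trigger boxes set CanChangeGravity on BP_Player on begin overlap.
; Their end-overlap events only cast, as the nodes that would clear the flag are unwired.
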(event OnComponentBeginOverlap(Box)
  (params (OverlappedComponent :type Primitive%20Component%20Object%20Reference) (OtherActor :type Actor%20Object%20Reference) (OtherComp :type Primitive%20Component%20Object%20Reference) (OtherBodyIndex :type Integer) (bFromSweep :type Boolean) (SweepResult :type Hit%20Result%20Structure%20%28by%20ref%29))
  (bind _asbp_player (Utilities|Casting|CastToBP_Player OtherActor))
  (Variables|/Game/Blueprints/BP_Player.BP_Player_C|SetCanChangeGravity _asbp_player true))

(event OnComponentBeginOverlap(Box1)
  (params (OverlappedComponent :type Primitive%20Component%20Object%20Reference) (OtherActor :type Actor%20Object%20Reference) (OtherComp :type Primitive%20Component%20Object%20Reference) (OtherBodyIndex :type Integer) (bFromSweep :type Boolean) (SweepResult :type Hit%20Result%20Structure%20%28by%20ref%29))
  (bind _asbp_player (Utilities|Casting|CastToBP_Player OtherActor))
  (Variables|/Game/Blueprints/BP_Player.BP_Player_C|SetCanChangeGravity _asbp_player true))

(event OnComponentHit(Cube)
  (params (HitComponent :type Primitive%20Component%20Object%20Reference) (OtherActor :type Actor%20Object%20Reference) (OtherComp :type Primitive%20Component%20Object%20Reference) (NormalImpulse :type Vector :default "0, 0, 0") (Hit :type Hit%20Result%20Structure%20%28by%20ref%29))
  (Sprite|SetFlipbook (Variables|Default|GetPaperFlipbook) "/Game/Blueprints/Floppa/FB_FloppaDPlatform.FB_FloppaDPlatform")
  (Utilities|FlowControl|Delay 0.3125)
  (Rendering|SetActorHiddenInGame true)
  (Utilities|FlowControl|Sequence
    (:then_1
      (Collision|SetCollisionEnabled (Variables|Default|GetCube) "NoCollision")
      (Audio|PlaySoundatLocation "/Game/Assets/SFX/SFX_PlatformDisappears.SFX_PlatformDisappears" "0, 0, 0" "0, 0, 0" 1.0 1.0 0.0 0 0 0))))

(event OnComponentEndOverlap(Box)
  (params (OverlappedComponent :type Primitive%20Component%20Object%20Reference) (OtherActor :type Actor%20Object%20Reference) (OtherComp :type Primitive%20Component%20Object%20Reference) (OtherBodyIndex :type Integer))
  (Utilities|Casting|CastToBP_Player OtherActor))

(event OnComponentEndOverlap(Box1)
  (params (OverlappedComponent :type Primitive%20Component%20Object%20Reference) (OtherActor :type Actor%20Object%20Reference) (OtherComp :type Primitive%20Component%20Object%20Reference) (OtherBodyIndex :type Integer))
  (Utilities|Casting|CastToBP_Player OtherActor))

(fn ConstructionScript)