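; BP_DFloor is a disappearing floor with a Paper2D flipbook visual.
; A hit on its Cube component switches the flipbook to FB_DFloorA and starts a fixed delay.
; The actor then hides and turns off collision on Cube, Cub and Cub1, with no logic to restore it.
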(event OnComponentHit(Cube)
  (params (HitComponent :type Primitive%20Component%20Object%20Reference) (OtherActor :type Actor%20Object%20Reference) (OtherComp :type Primitive%20Component%20Object%20Reference) (NormalImpulse :type Vector :default "0, 0, 0") (Hit :type Hit%20Result%20Structure%20%28by%20ref%29))
  (Sprite|SetFlipbook (Variables|Default|GetPaperFlipbook) "/Game/Assets/FB_DFloorA.FB_DFloorA")
  (Utilities|FlowControl|Delay 3.0)
  (Rendering|SetActorHiddenInGame true)
  (Utilities|FlowControl|Sequence
    (:then_0
      (Collision|SetCollisionEnabled (Variables|Default|GetCub) "NoCollision"))
    (:then_1
      (Collision|SetCollisionEnabled (Variables|Default|GetCube) "NoCollision"))
    (:then_2
      (Collision|SetCollisionEnabled (Variables|Default|GetCub1) "NoCollision"))))

(fn ConstructionScript)